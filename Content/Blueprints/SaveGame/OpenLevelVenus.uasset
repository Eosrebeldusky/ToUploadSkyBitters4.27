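; Level-exit trigger that marks Mercury as complete in the save game and opens the Venus level.
; When the 2DSideScrollerCharacter overlaps its collision component, it creates a SaveGameSkyBitters object and checks for an existing save slot.
; An existing save is loaded, flagged and rewritten before travel.
; Without one, it only saves the new object, without setting the flag or changing level.
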(event `self.CollisionComponent.OnComponentBeginOverlap`
  (params (OverlappedComponent :type "PrimitiveComponent Object Reference") (OtherActor :type "Actor Object Reference") (OtherComp :type "PrimitiveComponent Object Reference") (OtherBodyIndex :type Integer) (bFromSweep :type Boolean) (SweepResult :type "HitResult Structure (by ref)"))
  (cast `/Game/2DSideScrollerBP/Blueprints/2DSideScrollerCharacter` OtherActor)
  (bind _returnvalue (`GameplayStatics.CreateSaveGameObject` "/Game/Blueprints/SaveGame/SaveGameSkyBitters.SaveGameSkyBitters_C"))
  (bind _output_get (set `self.SaveGameSkyBittersRef` _returnvalue))
  (bind _returnvalue_2 (`GameplayStatics.DoesSaveGameExist` "SaveGameSkyBitters"))
  (if _returnvalue_2
    (bind _returnvalue_3 (`GameplayStatics.LoadGameFromSlot` "SaveGameSkyBitters"))
    (bind _assave_game_sky_bitters (cast `/Game/Blueprints/SaveGame/SaveGameSkyBitters` _returnvalue_3))
    (bind _output_get_2 (set `self.SaveGameSkyBittersInstance` _assave_game_sky_bitters))
    (set `/Game/Blueprints/SaveGame/SaveGameSkyBitters.LevelMercuryComplete` true _output_get_2)
    (`GameplayStatics.SaveGameToSlot` _output_get_2 "SaveGameSkyBitters")
    (`GameplayStatics.OpenLevel` "Venus")
    (else
      (`GameplayStatics.SaveGameToSlot` _output_get "SaveGameSkyBitters"))))

(fn `UserConstructionScript`)